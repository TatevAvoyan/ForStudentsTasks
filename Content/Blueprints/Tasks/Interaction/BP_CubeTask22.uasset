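; Task actor for an interaction exercise: a cube that starts and stops rotating on alternate left mouse clicks.
; On BeginPlay it binds to the spectator pawn's left-click dispatcher, and a FlipFlop switches between playing and stopping a Timeline.
; One Timeline track drives both roll and pitch.
; A macro, unused in the event graph, routes inputs to move, rotate and color calls, of which only RotateCube is defined here.
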(event Custom|RotateCube
  (bind _newtrack_2 (Timeline|Timeline Play)
    (:Update
      (Transformation|SetActorRotation (Math|Rotator|MakeRotator _newtrack_2 _newtrack_2 0.0)))))

(event Custom|OnMouseLeftButtonClicked_Event
  (Utilities|FlowControl|FlipFlop
    (:A
      (CallFunction|RotateCube))
    (:B
      (CallFunction|StopTimeline))))

(event Custom|StopTimeline
  (bind _newtrack_2 (Timeline|Timeline Stop)
    (:Update
      (Transformation|SetActorRotation (Math|Rotator|MakeRotator _newtrack_2 _newtrack_2 0.0)))))

(event EventBeginPlay
  (bind _asbp_spectator_pawn (Utilities|Casting|CastToBP_SpectatorPawn (Game|Player|GetPlayerPawn 0)))
  (EventDispatchers|AssignOnMouseLeftButtonClicked _asbp_spectator_pawn (delegate Custom|OnMouseLeftButtonClicked_Event)))

(fn ConstructionScript)