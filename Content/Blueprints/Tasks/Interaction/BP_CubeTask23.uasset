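; BP_CubeTask23 is an interaction task cube whose looping side-to-side movement and color animation are toggled by the spectator pawn's T-key event.
; A FlipFlop starts or stops two timelines that ping-pong by reversing at each end.
; One offsets the actor from its start location, the other drives the Color parameter of a dynamic material.
; A separate NewMacro routes inputs to movement, rotation and color events.
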(event Custom|ReverseCubeSide
  (bind (_direction _newtrack_2) (Timeline|Left/Right Reverse)
    (:Update
      (Transformation|SetActorLocation (+ (Variables|Default|GetStartLocation) _newtrack_2) false false))
    (:Finished
      (switch Utilities|FlowControl|Switch|SwitchonETimelineDirection _direction
        (:Forward
          (CallFunction|ReverseCubeSide))
        (:Backward
          (CallFunction|MoveCubeSide))))))

(event Custom|ChangeColor
  (bind (_direction _newtrack_0) (Timeline|ColorTimeline Play)
    (:Update
      (Rendering|Material|SetVectorParameterValue (Variables|Default|GetMaterialInstance) "Color" _newtrack_0 :!class /Script/Engine.MaterialInstanceDynamic))
    (:Finished
      (switch Utilities|FlowControl|Switch|SwitchonETimelineDirection _direction
        (:Forward
          (CallFunction|ReverseColor))
        (:Backward
          (CallFunction|ChangeColor))))))

(event Custom|OnInteractionKeyTPressed_Event
  (Utilities|FlowControl|FlipFlop
    (:A
      (CallFunction|MoveCubeSide)
      (CallFunction|ChangeColor))
    (:B
      (Audio|Components|Audio|Stop (Variables|Default|GetLeft/Right))
      (Audio|Components|Audio|Stop (Variables|Default|GetColorTimeline)))))

(event Custom|MoveCubeSide
  (bind (_direction _newtrack_2) (Timeline|Left/Right Play)
    (:Update
      (Transformation|SetActorLocation (+ (Variables|Default|GetStartLocation) _newtrack_2) false false))
    (:Finished
      (switch Utilities|FlowControl|Switch|SwitchonETimelineDirection _direction
        (:Forward
          (CallFunction|ReverseCubeSide))
        (:Backward
          (CallFunction|MoveCubeSide))))))

(event Custom|ReverseColor
  (bind (_direction _newtrack_0) (Timeline|ColorTimeline ReverseFromEnd)
    (:Update
      (Rendering|Material|SetVectorParameterValue (Variables|Default|GetMaterialInstance) "Color" _newtrack_0 :!class /Script/Engine.MaterialInstanceDynamic))
    (:Finished
      (switch Utilities|FlowControl|Switch|SwitchonETimelineDirection _direction
        (:Forward
          (CallFunction|ReverseColor))
        (:Backward
          (CallFunction|ChangeColor))))))

(event EventBeginPlay
  (bind _returnvalue (Rendering|Material|CreateDynamicMaterialInstance (Variables|Default|GetCube) 0 0 "None" :!class /Script/Engine.PrimitiveComponent))
  (Variables|Default|SetMaterialInstance _returnvalue)
  (Variables|Default|SetStartLocation (Transformation|GetActorLocation))
  (bind _asbp_spectator_pawn (Utilities|Casting|CastToBP_SpectatorPawn (Game|Player|GetPlayerPawn 0)))
  (EventDispatchers|AssignOnInteractionKeyTPressed _asbp_spectator_pawn (delegate Custom|OnInteractionKeyTPressed_Event)))

(fn ConstructionScript)