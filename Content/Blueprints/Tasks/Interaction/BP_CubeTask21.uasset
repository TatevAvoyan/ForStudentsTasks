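; BP_CubeTask21 is an interaction task cube that toggles a looping up-and-down motion.
; It binds to the spectator pawn's interaction key event, where a FlipFlop alternates between playing and stopping the UpDown timeline.
; The timeline offsets the cube from its start location and ping-pongs by reversing or replaying when finished.
; An uncalled macro routes inputs to move, rotate and color events, of which only MoveCubeUp is defined here.
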(event Custom|MoveCubeUp
  (bind (_direction _newtrack_2) (Timeline|Up/Down Play)
    (:Update
      (Transformation|SetActorLocation (+ (Variables|Default|GetStartLocation) _newtrack_2) false false))
    (:Finished
      (switch Utilities|FlowControl|Switch|SwitchonETimelineDirection _direction
        (:Forward
          (CallFunction|ReverseCubeDown))
        (:Backward
          (CallFunction|MoveCubeUp))))))

(event Custom|ReverseCubeDown
  (bind (_direction _newtrack_2) (Timeline|Up/Down Reverse)
    (:Update
      (Transformation|SetActorLocation (+ (Variables|Default|GetStartLocation) _newtrack_2) false false))
    (:Finished
      (switch Utilities|FlowControl|Switch|SwitchonETimelineDirection _direction
        (:Forward
          (CallFunction|ReverseCubeDown))
        (:Backward
          (CallFunction|MoveCubeUp))))))

(event Custom|InteractionKeyPressed
  (Utilities|FlowControl|FlipFlop
    (:A
      (CallFunction|MoveCubeUp))
    (:B
      (CallFunction|StopTimeline))))

(event Custom|StopTimeline
  (bind (_direction _newtrack_2) (Timeline|Up/Down Stop)
    (:Update
      (Transformation|SetActorLocation (+ (Variables|Default|GetStartLocation) _newtrack_2) false false))
    (:Finished
      (switch Utilities|FlowControl|Switch|SwitchonETimelineDirection _direction
        (:Forward
          (CallFunction|ReverseCubeDown))
        (:Backward
          (CallFunction|MoveCubeUp))))))

(event EventBeginPlay
  (Variables|Default|SetStartLocation (Transformation|GetActorLocation))
  (bind _asbp_spectator_pawn (Utilities|Casting|CastToBP_SpectatorPawn (Game|Player|GetPlayerPawn 0)))
  (EventDispatchers|BindEventtoInterastionKeyPressed _asbp_spectator_pawn (delegate Custom|InteractionKeyPressed)))

(fn ConstructionScript)