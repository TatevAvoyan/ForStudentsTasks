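; Task cube actor that moves up and down in an endless loop from the location it has at BeginPlay.
; The UpDown timeline offsets that start location, and its Finished output checks direction to alternate between reversing and replaying.
; An unused macro routes Default/Up, Side, Rotate and Color inputs to movement, rotation and color calls, of which only MoveCubeUp is defined here.
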(event Custom|MoveCubeUp
  (bind (_direction _newtrack_2) (Timeline|Up/Down PlayFromStart)
    (:Update
      (Transformation|SetActorLocation (+ (Variables|Default|GetStartLocation) _newtrack_2) false false))
    (:Finished
      (switch Utilities|FlowControl|Switch|SwitchonETimelineDirection _direction
        (:Forward
          (CallFunction|ReverseCubeDown))
        (:Backward
          (CallFunction|MoveCubeUp))))))

(event Custom|ReverseCubeDown
  (bind (_direction _newtrack_2) (Timeline|Up/Down Reverse)
    (:Update
      (Transformation|SetActorLocation (+ (Variables|Default|GetStartLocation) _newtrack_2) false false))
    (:Finished
      (switch Utilities|FlowControl|Switch|SwitchonETimelineDirection _direction
        (:Forward
          (CallFunction|ReverseCubeDown))
        (:Backward
          (CallFunction|MoveCubeUp))))))

(event EventBeginPlay
  (Variables|Default|SetStartLocation (Transformation|GetActorLocation))
  (CallFunction|MoveCubeUp))

(fn ConstructionScript)