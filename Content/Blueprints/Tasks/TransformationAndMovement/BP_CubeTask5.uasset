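; Task cube actor that animates its scale from BeginPlay, despite event names that suggest vertical movement.
; It stores the starting scale, then the UpDown timeline adds its track value to it on each update.
; A reverse event and direction switch exist, but the switch is disconnected, so nothing here triggers reversal.
; An uncalled NewMacro routes inputs to move, rotate and color calls, of which only MoveCubeUp is defined here.
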(event Custom|MoveCubeUp
  (bind (_direction _newtrack_2) (Timeline|Up/Down PlayFromStart)
    (:Update
      (Transformation|SetRelativeScale3D (Variables|Default|GetCube) (+ (Variables|Default|GetStartScale) _newtrack_2)))))

(event Custom|ReverseCubeDown
  (bind (_direction _newtrack_2) (Timeline|Up/Down Reverse)
    (:Update
      (Transformation|SetRelativeScale3D (Variables|Default|GetCube) (+ (Variables|Default|GetStartScale) _newtrack_2)))))

(event EventBeginPlay
  (Variables|Default|SetStartScale (Variables|/Script/Engine.SceneComponent|GetRelativeScale3D (Variables|Default|GetCube)))
  (CallFunction|MoveCubeUp))

(fn ConstructionScript)