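; BP_CubeTask is a movement and transformation exercise actor for a cube.
; On Tick it eases with a swept VInterpTo toward a point above its start, then lowers the target by the same step whenever reached, so it keeps descending.
; Timeline events ping-pong vertical and sideways movement, rotation and material color by reversing on finish.
; Their flag-driven macro dispatch and dynamic material setup are disconnected, so only the interpolation runs by itself.
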(event Custom|MoveCubeUp
  (bind (_direction _newtrack_2) (Timeline|Up/Down PlayFromStart)
    (:Update
      (Transformation|SetActorLocation (+ (Variables|Default|GetStartLocation) _newtrack_2) false false))
    (:Finished
      (switch Utilities|FlowControl|Switch|SwitchonETimelineDirection _direction
        (:Forward
          (CallFunction|ReverseCubeDown))
        (:Backward
          (CallFunction|MoveCubeUp))))))

(event Custom|ReverseCubeDown
  (bind (_direction _newtrack_2) (Timeline|Up/Down Reverse)
    (:Update
      (Transformation|SetActorLocation (+ (Variables|Default|GetStartLocation) _newtrack_2) false false))
    (:Finished
      (switch Utilities|FlowControl|Switch|SwitchonETimelineDirection _direction
        (:Forward
          (CallFunction|ReverseCubeDown))
        (:Backward
          (CallFunction|MoveCubeUp))))))

(event Custom|RotateCube
  (bind (_direction _newtrack_2) (Timeline|Timeline Play)
    (:Update
      (Transformation|SetActorRotation (Math|Rotator|MakeRotator _newtrack_2 _newtrack_2 _newtrack_2)))
    (:Finished
      (switch Utilities|FlowControl|Switch|SwitchonETimelineDirection _direction
        (:Forward
          (CallFunction|ReverseRotation))
        (:Backward
          (CallFunction|RotateCube))))))

(event Custom|ReverseRotation
  (bind (_direction _newtrack_2) (Timeline|Timeline ReverseFromEnd)
    (:Update
      (Transformation|SetActorRotation (Math|Rotator|MakeRotator _newtrack_2 _newtrack_2 _newtrack_2)))
    (:Finished
      (switch Utilities|FlowControl|Switch|SwitchonETimelineDirection _direction
        (:Forward
          (CallFunction|ReverseRotation))
        (:Backward
          (CallFunction|RotateCube))))))

(event Custom|ChangeColor
  (bind (_direction _newtrack_0) (Timeline|Timeline_0 Play)
    (:Update
      (Rendering|Material|SetVectorParameterValue (Variables|Default|GetMaterialInstance) "Color" _newtrack_0 :!class /Script/Engine.MaterialInstanceDynamic))
    (:Finished
      (switch Utilities|FlowControl|Switch|SwitchonETimelineDirection _direction
        (:Forward
          (CallFunction|ReverseColor))
        (:Backward
          (CallFunction|ChangeColor))))))

(event Custom|MoveCubeSide
  (bind (_direction _newtrack_2) (Timeline|Left/Right PlayFromStart)
    (:Update
      (Transformation|SetActorLocation (+ (Variables|Default|GetStartLocation) _newtrack_2) false false))
    (:Finished
      (switch Utilities|FlowControl|Switch|SwitchonETimelineDirection _direction
        (:Forward
          (CallFunction|ReverseCubeSide))
        (:Backward
          (CallFunction|MoveCubeSide))))))

(event Custom|ReverseCubeSide
  (bind (_direction _newtrack_2) (Timeline|Left/Right ReverseFromEnd)
    (:Update
      (Transformation|SetActorLocation (+ (Variables|Default|GetStartLocation) _newtrack_2) false false))
    (:Finished
      (switch Utilities|FlowControl|Switch|SwitchonETimelineDirection _direction
        (:Forward
          (CallFunction|ReverseCubeSide))
        (:Backward
          (CallFunction|MoveCubeSide))))))

(event Custom|ReverseColor
  (bind (_direction _newtrack_0) (Timeline|Timeline_0 ReverseFromEnd)
    (:Update
      (Rendering|Material|SetVectorParameterValue (Variables|Default|GetMaterialInstance) "Color" _newtrack_0 :!class /Script/Engine.MaterialInstanceDynamic))
    (:Finished
      (switch Utilities|FlowControl|Switch|SwitchonETimelineDirection _direction
        (:Forward
          (CallFunction|ReverseColor))
        (:Backward
          (CallFunction|ChangeColor))))))

(event EventBeginPlay
  (Variables|Default|SetStartLocation (Transformation|GetActorLocation))
  (Variables|Default|SetTargetLocation (+ (Variables|Default|GetStartLocation) "0.000000,0.000000,100.000000")))

(event EventTick
  (params (DeltaSeconds :type Float%20%28single-precision%29))
  (if (not (Math|Float|NearlyEqual(Float) (.z (Variables|Default|GetTargetLocation)) (.z (Transformation|GetActorLocation)) 5.0))
    (Transformation|SetActorLocation (Math|Interpolation|VInterpTo (Transformation|GetActorLocation) (Variables|Default|GetTargetLocation) DeltaSeconds 0.5) true false)
    (else
      (Variables|Default|SetTargetLocation (- (Variables|Default|GetTargetLocation) "0.000000,0.000000,100.000000")))))

(fn ConstructionScript)