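; BP_CubeTask1 is a transformation-and-movement task actor that rotates itself on the roll axis.
; BeginPlay calls RotateCube, which plays a Timeline that sets the actor's roll on each update.
; ReverseRotation is an empty stub, and the Forward/Backward branch choosing between the two events is never executed.
; An unused macro, NewMacro, maps separate exec inputs to move up, move sideways, rotate or change color, defaulting to up.
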(event Custom|RotateCube
  (bind _newtrack_2 (Timeline|Timeline Play)
    (:Update
      (Transformation|SetActorRotation (Math|Rotator|MakeRotator _newtrack_2 0.0 0.0)))))

(event Custom|ReverseRotation)

(event EventBeginPlay
  (CallFunction|RotateCube))

(fn ConstructionScript)